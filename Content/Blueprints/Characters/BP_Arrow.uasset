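; Arrow projectile actor that detaches on ShootArrow and launches forward at a speed interpolated from the shot's charge.
; While simulating, Tick integrates mass-scaled gravity by hand and line-traces each step to catch hits between frames.
; Hits either consume a punch-through count and continue, or stop and destroy the arrow.
; It also has a lifetime check and event hooks for spawn, stat changes and impacts, mostly empty or debug prints.
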(event `self.ReceiveTick`
  (params (DeltaSeconds :type "Float (single-precision)"))
  (bind _returnvalue (+ (`self.CurrentPosition`) (* (`self.CurrentVelocity`) DeltaSeconds)))
  ; Arrow Physics Calculations
  (if (`self.IsSimulating`)
    (`self.LifetimeCountdown` DeltaSeconds)
    (bind _currentpositionoutput (`self.ApplyPhysics` DeltaSeconds))
    (bind _outhit (`KismetSystemLibrary.LineTraceSingle` _currentpositionoutput _returnvalue "TraceTypeQuery1"))
    (bind (_bblockinghit _binitialoverlap _time _distance _location) (`GameplayStatics.BreakHitResult` _outhit))
    (if _bblockinghit
      (`self.HitLocation` _location _returnvalue)
      (else
        (`self.K2_SetActorLocation` _returnvalue)))))

(event `ShootArrow`
  (bind _chargefuckery (`self.ChargeFuckery`))
  (bind _returnvalue (`KismetMathLibrary.FClamp` (/ _chargefuckery (`self.MaxCharge`))))
  (bind _returnvalue_2 (`KismetMathLibrary.Lerp` (`self.MinSpeed`) (`self.MaxSpeed`) _returnvalue))
  ; Shoot Mechanic (takes Player's input charge and makes it something usable)
  (`self.K2_DetachFromActor` "KeepWorld" "KeepWorld" "KeepWorld")
  (bind _output_get (set `self.CurrentVelocity` (* (`self.GetActorForwardVector`) _returnvalue_2)))
  (set `self.IsSimulating` true)
  (`KismetSystemLibrary.PrintString` (`KismetStringLibrary.Conv_VectorToString` _output_get) true true (struct :`R` 1.0 :`G` 0.878583 :`A` 1.0))
  (`KismetSystemLibrary.PrintString` (`KismetStringLibrary.Conv_DoubleToString` _returnvalue_2) true true (struct :`G` 1.0 :`B` 0.108827 :`A` 1.0))
  (`KismetSystemLibrary.PrintString` (`KismetStringLibrary.Conv_DoubleToString` _chargefuckery) true true (struct :`R` 0.204699 :`G` 0.254008 :`B` 1.0 :`A` 1.0))
  (`KismetSystemLibrary.PrintString` (`KismetStringLibrary.Conv_DoubleToString` _returnvalue) true true (struct :`R` 1.0 :`B` 0.047629 :`A` 1.0)))

(event `self.ReceiveBeginPlay`
  ; Misc Stuff
  (set `self.IsSimulating` false)
  (`self.OnArrowSpawned`)
  (`self.ModifyArrowStats`))

(event `ShotTooSoon`
  ; Misc Stuff
  (`self.K2_DestroyActor`))

(event `OnArrowHit`
  ; Misc Stuff
  (`KismetSystemLibrary.PrintString` "Arrow has hit something"))

(event `OnArrowSpawned`
  ; Misc Stuff
  (`KismetSystemLibrary.PrintString` "ArrowSpawned"))

(event `ModifyArrowStats`
  ; Misc Stuff
)

(event `OnImpactResolved`
  ; Misc Stuff
)

(fn `ApplyPhysics`
  (params (DeltaTimeInput :type "Float (single-precision)"))
  (returns (CurrentPositionOutput :type "Vector Structure"))
  (set `self.Acceleration` (* (* (`KismetMathLibrary.MakeVector` 0.0 0.0 -980.0) (`self.GravityScale`)) (`self.Mass`)))
  (set `self.CurrentVelocity` (+ (`self.CurrentVelocity`) (* (`self.Acceleration`) DeltaTimeInput)))
  (bind _output_get (set `self.CurrentPosition` (`self.K2_GetActorLocation`)))
  (return _output_get))

(fn `HitLocation`
  (params (HitLocation :type "Vector Structure") (NewLocation :type "Vector Structure"))
  (`/Engine/EditorBlueprintResources/StandardMacros.CompareInt` (`self.PunchTrough`)
    (:`>`
      (`self.K2_SetActorLocation` NewLocation)
      (`self.OnArrowHit`)
      (set `self.PunchTrough` (- (`self.PunchTrough`) 1))
      (`self.OnImpactResolved `))
    (:`==`
      (`self.K2_SetActorLocation` HitLocation :!label _label)
      (`self.OnArrowHit`)
      (set `self.IsSimulating` false)
      (`self.OnImpactResolved `)
      (`self.K2_DestroyActor`))
    (:`<`
      (goto _label))))

(fn `LifetimeCountdown`
  (params (DeltaTimeInput :type "Float (double-precision)"))
  (`/Engine/EditorBlueprintResources/StandardMacros.CompareFloat` (+ (`self.LifeTimer`) DeltaTimeInput) (`self.LifeTime`)
    (:`>`
      _)
    (:`==`
      _)
    (:`<`
      (return)))
  (`self.K2_DestroyActor`))

(fn `UserConstructionScript`)