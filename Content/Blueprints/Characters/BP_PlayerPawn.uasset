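; Player character for a bow-style shooter, with Enhanced Input movement, invertible look, jump, a launch-based dash and a five-slot arrow quiver.
; Shooting spawns the equipped arrow on the spawn point, grows its charge and scale along the ChargeWeapon timeline, then fires on release or at full charge.
; Quiver inputs select or cycle CurrentArrow, which Tick maps to the equipped projectile, though every slot currently resolves to BP_Arrow.
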(event `EnhancedInput|/Game/Blueprints/InputMaps/Actions/IA_Shoot`
  (params (ActionValue :type Boolean) (ElapsedSeconds :type "Float (double-precision)") (TriggeredSeconds :type "Float (double-precision)") (InputAction :type "InputAction Object Reference" :default "/Game/Blueprints/InputMaps/Actions/IA_Shoot.IA_Shoot"))
  (bind _projectile (`self.Projectile`))
  (bind _projectilespawnpoint (`self.ProjectileSpawnPoint`))
  (bind _chargebullshit (`self.ChargeBullshit`))
  ; Shooting mechanics (Spawns Projectile and applies charge level to the projectile)
  (:`Started`
    (set `self.WasHeld?` true)
    (`KismetSystemLibrary.PrintString` "Held")
    (bind _returnvalue (`|SpawnActorFromClass` (`self.EquipedProjectile`) (`KismetMathLibrary.MakeTransform` (`SceneComponent.K2_GetComponentLocation` _projectilespawnpoint) (`SceneComponent.K2_GetComponentRotation` _projectilespawnpoint)) "Undefined" "MultiplyWithRoot" null (`self.ChargeBullshit`) null))
    (bind _output_get (set `self.Projectile` _returnvalue))
    (`self.K2_AttachToComponent` _output_get (`self.ProjectileSpawnPoint`) "None" "KeepWorld" "KeepWorld" "KeepWorld" true)
    (`Timeline|ChargeWeapon` :!via `PlayFromStart` :!label _label
      (:`Charge`
        (if (< _chargebullshit 10.0)
          (bind _output_get_2 (set `self.ChargeBullshit` (+ _chargebullshit 0.5)))
          (bind _output_get_3 (set `/Game/Blueprints/Characters/BP_Arrow.ChargeFuckery` _output_get_2 _projectile))
          (`self.SetActorScale3D` _projectile (`KismetMathLibrary.VLerp` (`self.GetActorScale3D` _projectile) (`KismetMathLibrary.Conv_DoubleToVector` (/ _output_get_3 4.0)) 0.1))
          (else
            (`KismetSystemLibrary.Delay` 0.2)
            (`/Game/Blueprints/Characters/BP_Arrow.ShootArrow` (`self.Projectile`))
            (`self.StopCharging`))))))
  (:`Completed`
    (if (`self.WasHeld?`)
      (`KismetSystemLibrary.PrintString` "released"))
    (set `self.WasHeld?` false)
    (`KismetSystemLibrary.Delay` 0.2)
    (`/Game/Blueprints/Characters/BP_Arrow.ShootArrow` (`self.Projectile`))
    (`self.StopCharging`)))

(event `StopCharging`
  ; Shooting mechanics (Spawns Projectile and applies charge level to the projectile)
  (set `self.ChargeBullshit` 0.0)
  (goto _label :!via `Stop`))

(event `EnhancedInput|/Game/Blueprints/InputMaps/Actions/IA_Look`
  (params (ActionValue :type "Vector2D Structure") (ElapsedSeconds :type "Float (double-precision)") (TriggeredSeconds :type "Float (double-precision)") (InputAction :type "InputAction Object Reference" :default "/Game/Blueprints/InputMaps/Actions/IA_Look.IA_Look"))
  (bind (_x _y) (`KismetMathLibrary.BreakVector2D` ActionValue))
  (bind (_x_2 _y_2) (`KismetMathLibrary.BreakVector2D` (* ActionValue (-1.0 -1.0))))
  ; Look Logic
  (:`Triggered`
    (if (`self.Inverted?`)
      (`self.Aim` _x_2 _y_2)
      (else
        (`self.Aim` _x _y)))))

(event `EnhancedInput|/Game/Blueprints/InputMaps/Actions/IA_CycleArrowUP`
  (params (ActionValue :type "Vector2D Structure") (ElapsedSeconds :type "Float (double-precision)") (TriggeredSeconds :type "Float (double-precision)") (InputAction :type "InputAction Object Reference" :default "/Game/Blueprints/InputMaps/Actions/IA_CycleArrowUP.IA_CycleArrowUP"))
  ; Quiver
  (:`Triggered`
    (`/Engine/EditorBlueprintResources/StandardMacros.CompareFloat` (`KismetMathLibrary.BreakVector2D` ActionValue)
      (:`>`
        (`KismetSystemLibrary.PrintString` "Cycle Up Works")
        (`self.CycleArrow` 1))
      (:`<`
        (`KismetSystemLibrary.PrintString` "Cycle Down Works")
        (`self.CycleArrow` -1)))
    (`KismetSystemLibrary.PrintString` (`KismetStringLibrary.Conv_IntToString` (`self.CurrentArrow`)) :!label _label_2)))

(event `EnhancedInput|/Game/Blueprints/InputMaps/Actions/IA_BasicArrow`
  (params (ActionValue :type Boolean) (ElapsedSeconds :type "Float (double-precision)") (TriggeredSeconds :type "Float (double-precision)") (InputAction :type "InputAction Object Reference" :default "/Game/Blueprints/InputMaps/Actions/IA_BasicArrow.IA_BasicArrow"))
  ; Quiver
  (:`Triggered`
    (`KismetSystemLibrary.PrintString` "Cycle 0 Works")
    (set `self.CurrentArrow` 0)
    (goto _label_2)))

(event `self.ReceiveBeginPlay`
  ; Adds Mapping Context
  (`KismetSystemLibrary.PrintString` "Character Spawned")
  (`EnhancedInputSubsystemInterface.AddMappingContext` (pcsubsystem `EnhancedInputLocalPlayerSubsystem` (`GameplayStatics.GetPlayerController` 0)) "/Game/Blueprints/InputMaps/IMC_Player.IMC_Player" 0 (struct)))

(event `EnhancedInput|/Game/Blueprints/InputMaps/Actions/IA_Jump`
  (params (ActionValue :type Boolean) (ElapsedSeconds :type "Float (double-precision)") (TriggeredSeconds :type "Float (double-precision)") (InputAction :type "InputAction Object Reference" :default "/Game/Blueprints/InputMaps/Actions/IA_Jump.IA_Jump"))
  ; Jump Logic
  (:`Started`
    (`self.Jump`)))

(event `EnhancedInput|/Game/Blueprints/InputMaps/Actions/IA_ElectricArrow`
  (params (ActionValue :type Boolean) (ElapsedSeconds :type "Float (double-precision)") (TriggeredSeconds :type "Float (double-precision)") (InputAction :type "InputAction Object Reference" :default "/Game/Blueprints/InputMaps/Actions/IA_ElectricArrow.IA_ElectricArrow"))
  ; Quiver
  (:`Triggered`
    (`KismetSystemLibrary.PrintString` "Cycle 1 Works")
    (set `self.CurrentArrow` 1)
    (goto _label_2)))

(event `EnhancedInput|/Game/Blueprints/InputMaps/Actions/IA_FireArrow`
  (params (ActionValue :type Boolean) (ElapsedSeconds :type "Float (double-precision)") (TriggeredSeconds :type "Float (double-precision)") (InputAction :type "InputAction Object Reference" :default "/Game/Blueprints/InputMaps/Actions/IA_FireArrow.IA_FireArrow"))
  ; Quiver
  (:`Triggered`
    (`KismetSystemLibrary.PrintString` "Cycle 2 Works")
    (set `self.CurrentArrow` 2)
    (goto _label_2)))

(event `EnhancedInput|/Game/Blueprints/InputMaps/Actions/IA_IceArrow`
  (params (ActionValue :type Boolean) (ElapsedSeconds :type "Float (double-precision)") (TriggeredSeconds :type "Float (double-precision)") (InputAction :type "InputAction Object Reference" :default "/Game/Blueprints/InputMaps/Actions/IA_IceArrow.IA_IceArrow"))
  ; Quiver
  (:`Triggered`
    (`KismetSystemLibrary.PrintString` "Cycle 3 Works")
    (set `self.CurrentArrow` 3)
    (goto _label_2)))

(event `EnhancedInput|/Game/Blueprints/InputMaps/Actions/IA_VortexArrow`
  (params (ActionValue :type Boolean) (ElapsedSeconds :type "Float (double-precision)") (TriggeredSeconds :type "Float (double-precision)") (InputAction :type "InputAction Object Reference" :default "/Game/Blueprints/InputMaps/Actions/IA_VortexArrow.IA_VortexArrow"))
  ; Quiver
  (:`Triggered`
    (`KismetSystemLibrary.PrintString` "Cycle 4 Works")
    (set `self.CurrentArrow` 4)
    (goto _label_2)))

(event `EnhancedInput|/Game/Blueprints/InputMaps/Actions/IA_Move`
  (params (ActionValue :type "Vector2D Structure") (ElapsedSeconds :type "Float (double-precision)") (TriggeredSeconds :type "Float (double-precision)") (InputAction :type "InputAction Object Reference" :default "/Game/Blueprints/InputMaps/Actions/IA_Move.IA_Move"))
  (bind (_x _y) (`KismetMathLibrary.BreakVector2D` ActionValue))
  (bind _movespeed (`self.MoveSpeed`))
  (bind _returnvalue (`KismetMathLibrary.MakeRotator` 0.0 0.0 (.yaw (`self.GetControlRotation`))))
  ; IMC Movement logic
  (:`Triggered`
    (`self.AddMovementInput` (`KismetMathLibrary.GetForwardVector` _returnvalue) (* _y _movespeed))
    (`self.AddMovementInput` (`KismetMathLibrary.GetRightVector` _returnvalue) (* _x _movespeed))))

(event `self.ReceiveTick`
  (params (DeltaSeconds :type "Float (single-precision)"))
  ; Quiver
  (switch `int` (`self.CurrentArrow`)
    (:`0`
      (set `self.EquipedProjectile` "/Game/Blueprints/Characters/BP_Arrow.BP_Arrow_C"))
    (:`1`
      (set `self.EquipedProjectile` "/Game/Blueprints/Characters/BP_Arrow.BP_Arrow_C"))
    (:`2`
      (set `self.EquipedProjectile` "/Game/Blueprints/Characters/BP_Arrow.BP_Arrow_C"))
    (:`3`
      (set `self.EquipedProjectile` "/Game/Blueprints/Characters/BP_Arrow.BP_Arrow_C"))
    (:`4`
      (set `self.EquipedProjectile` "/Game/Blueprints/Characters/BP_Arrow.BP_Arrow_C"))))

(event `EnhancedInput|/Game/Blueprints/InputMaps/Actions/IA_Dash`
  (params (ActionValue :type Boolean) (ElapsedSeconds :type "Float (double-precision)") (TriggeredSeconds :type "Float (double-precision)") (InputAction :type "InputAction Object Reference" :default "/Game/Blueprints/InputMaps/Actions/IA_Dash.IA_Dash"))
  (bind _returnvalue (`self.GetVelocity`))
  ; IMC Dash Logic
  (:`Started`
    (if (`self.CanDash?`)
      (`self.LaunchCharacter` (0.0 0.0 200.0))
      (`KismetSystemLibrary.Delay` 0.2)
      (`self.LaunchCharacter` (* _returnvalue (4.0 4.0 1.0)))
      (set `self.CanDash?` false)
      (`KismetSystemLibrary.Delay` 0.2)
      (`self.LaunchCharacter` (* _returnvalue (-1.0 -1.0 0.0)))
      (`KismetSystemLibrary.Delay` 0.5)
      (set `self.CanDash?` true))))

(fn `Aim`
  (params (Yaw :type "Float (double-precision)") (Pitch :type "Float (double-precision)"))
  (bind _looksensitivity (`self.LookSensitivity`))
  (`self.AddControllerYawInput` (* Yaw _looksensitivity))
  (`SceneComponent.K2_AddRelativeRotation` (`self.Camera`) (`KismetMathLibrary.MakeRotator` 0.0 (* Pitch _looksensitivity)) false false))

(fn `CycleArrow`
  (params (CycleAmount :type Integer))
  (bind _returnvalue (+ (`self.CurrentArrow`) CycleAmount))
  (`/Engine/EditorBlueprintResources/StandardMacros.CompareInt` _returnvalue
    (:`>`
      (`/Engine/EditorBlueprintResources/StandardMacros.CompareInt` _returnvalue 4 :!label _label
        (:`>`
          (set `self.CurrentArrow` 0))
        (:`==`
          (set `self.CurrentArrow` _returnvalue :!label _label_2))
        (:`<`
          (goto _label_2))))
    (:`==`
      (goto _label))
    (:`<`
      (set `self.CurrentArrow` 4)))
  (return))

(fn `QuiverChecker`)

(fn `SpawnProjectile`
  (params (ProjectileClass :type "/Game/Blueprints/Characters/BP_Arrow Class Reference") (ChargePercent :type "Float (double-precision)"))
  (returns (OutputPin :type "/Game/Blueprints/Characters/BP_Arrow Object Reference"))
  (bind _projectilespawnpoint (`self.ProjectileSpawnPoint`))
  (bind _returnvalue (`|SpawnActorFromClass` ProjectileClass (`KismetMathLibrary.MakeTransform` (`SceneComponent.K2_GetComponentLocation` _projectilespawnpoint) (`SceneComponent.K2_GetComponentRotation` _projectilespawnpoint)) "Undefined" "MultiplyWithRoot" null ChargePercent null))
  (bind _output_get (set `self.Projectile` _returnvalue))
  (`self.K2_AttachToComponent` (`self.ProjectileSpawnPoint`) "None" "KeepWorld" "KeepWorld" "KeepWorld")
  (return _output_get))

(fn `UserConstructionScript`)